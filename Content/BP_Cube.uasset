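; BP_Cube is a cube actor configured by a Color (red, blue or green) and a Weight (light, medium or heavy).
; The construction script passes Color to the ColorCube member, tints a dynamic M_Solid material instance to match and scales the actor by weight class.
; On BeginPlay, the same weight class sets a mass override on the static mesh, so heavier cubes are also larger.
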(event EventBeginPlay
  (bind _staticmesh (Variables|Default|GetStaticMesh))
  (switch Utilities|FlowControl|Switch|SwitchonEWeightClass (Variables|Default|GetWeight)
    (:Weight_Light
      (Class|PrimitiveComponent|SetMassOverrideinKg _staticmesh "None" 1e+01 true))
    (:Weight_Medium
      (Class|PrimitiveComponent|SetMassOverrideinKg _staticmesh "None" 3e+01 true))
    (:Weight_Heavy
      (Class|PrimitiveComponent|SetMassOverrideinKg _staticmesh "None" 5e+01 true))))

(fn ConstructionScript
  (bind _returnvalue (Rendering|Material|CreateDynamicMaterialInstance "/Game/LevelPrototyping/Materials/M_Solid.M_Solid" "None" "None" :!class /Script/Engine.KismetMaterialLibrary))
  (bind _output_get (Variables|Default|SetMaterial _returnvalue))
  (Rendering|Material|SetMaterial (Variables|Default|GetStaticMesh) 0 _output_get)
  (bind _output_get_2 (Variables|/Script/HelloCpp.ColorCube|SetColor (Variables|Default|GetColorCube) (Variables|Default|GetColor)))
  (switch Utilities|FlowControl|Switch|SwitchonEColorType _output_get_2
    (:Color_Red
      (Rendering|Material|SetVectorParameterValue (Variables|Default|GetMaterial) "Base Color" (Variables|Default|GetRed) :!class /Script/Engine.MaterialInstanceDynamic))
    (:Color_Blue
      (Rendering|Material|SetVectorParameterValue (Variables|Default|GetMaterial) "Base Color" (Variables|Default|GetBlue) :!class /Script/Engine.MaterialInstanceDynamic))
    (:Color_Green
      (Rendering|Material|SetVectorParameterValue (Variables|Default|GetMaterial) "Base Color" (Variables|Default|GetGreen) :!class /Script/Engine.MaterialInstanceDynamic)))
  (switch Utilities|FlowControl|Switch|SwitchonEWeightClass (Variables|Default|GetWeight)
    (:Weight_Light
      (Transformation|SetActorScale3D "0.700000,0.700000,0.700000"))
    (:Weight_Medium
      (Transformation|SetActorScale3D "0.900000,0.900000,0.900000"))
    (:Weight_Heavy
      (Transformation|SetActorScale3D "1.200000,1.200000,1.200000"))))