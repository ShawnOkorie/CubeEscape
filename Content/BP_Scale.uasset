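; BP_Scale is a weight readout that displays the current load against the weight required to open a door.
; Each Tick it rewrites its TextRender as "total kg / required kg".
; It reads TotalWeight and RequiredWeight from the Door's OpenDoor member when Door is valid, otherwise from the Wall's WallDoor, with no validity check on Wall.
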(event EventTick
  (params (DeltaSeconds :type Float%20%28single-precision%29))
  (bind _textrender (Variables|Default|GetTextRender))
  (bind _wall (Variables|Default|GetWall))
  (bind _door (Variables|Default|GetDoor))
  (bind _opendoor (Variables|/Game/BP_Door.BP_Door_C|GetOpenDoor _door))
  (bind _walldoor (Variables|/Game/BP_Wall.BP_Wall_C|GetWallDoor _wall))
  (Utilities|IsValid _door
    (:Is%20Valid
      (Rendering|Components|TextRender|SetText _textrender (Utilities|Text|ToText(String) (Utilities|String|Append (Utilities|String|ToString(Integer) (Class|KismetMathLibrary|ToInt64(Float) (Variables|/Script/HelloCpp.OpenDoor|GetTotalWeight _opendoor))) " kg / " (Utilities|String|ToString(Integer) (Class|KismetMathLibrary|ToInt64(Float) (Variables|/Script/HelloCpp.OpenDoor|GetRequiredWeight _opendoor))) " kg"))))
    (:Is%20Not%20Valid
      (Rendering|Components|TextRender|SetText _textrender (Utilities|Text|ToText(String) (Utilities|String|Append (Utilities|String|ToString(Integer) (Class|KismetMathLibrary|ToInt64(Float) (Variables|/Script/HelloCpp.WallDoor|GetTotalWeight _walldoor))) " kg / " (Utilities|String|ToString(Integer) (Class|KismetMathLibrary|ToInt64(Float) (Variables|/Script/HelloCpp.WallDoor|GetRequiredWeight _walldoor))) " kg"))))))

(fn ConstructionScript)